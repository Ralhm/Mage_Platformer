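; BP_FloatingEnemy is an enemy that shows a text indicator when the player can grapple it.
; It caches the PlayerCharacter on BeginPlay, then on Tick, while not the player's look target, turns the text toward the player camera and calls SetCanGrappleEnemy on the player.
; Success toggles the text and CurrentGrappleTarget each tick rather than holding them on; failure hides the text and clears the flag.
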(event EventBeginPlay
  (bind _asplayer_character (Utilities|Casting|CastToPlayerCharacter (Game|GetPlayerCharacter 0)))
  (Variables|Default|SetPlayerRef _asplayer_character))

(event Collision|EventActorBeginOverlap
  (params (OtherActor :type Actor%20Object%20Reference)))

(event EventTick
  (params (DeltaSeconds :type Float%20%28single-precision%29))
  (bind _playerref (Variables|Default|GetPlayerRef))
  (bind _textrender (Variables|Default|GetTextRender))
  (if (not (== (Variables|/Script/CombatGame.PlayerCharacter|GetCurrentLookTarget _playerref) self))
    (Transformation|SetWorldRotation (Variables|Default|GetTextRender) (Math|Conversions|RotationFromXVector (- (Transformation|GetWorldLocation (Variables|/Script/CombatGame.PlayerCharacter|GetCamera _playerref)) (Transformation|GetActorLocation))) false false)
    (bind _returnvalue (Class|PlayerCharacter|SetCanGrappleEnemy (Variables|Default|GetPlayerRef) self true))
    (if _returnvalue
      (if (not (Variables|Default|GetCurrentGrappleTarget))
        (Development|SetHiddeninGame _textrender false false)
        (Variables|Default|SetCurrentGrappleTarget true)
        (else
          (Development|SetHiddeninGame _textrender true false :!label _label)
          (Variables|Default|SetCurrentGrappleTarget false)))
      (else
        (goto _label)))))

(fn ConstructionScript)